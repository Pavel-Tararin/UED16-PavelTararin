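; BP_TestA is a test Blueprint that exercises custom events and functions with mixed parameter types.
; BeginPlay fires a custom event twice, which prints its bool parameter in a color chosen by that value.
; NewFunction_0 checks the first array element, then calls both custom events and itself recursively with false, though nothing else shown calls it.
; The remaining events, function and construction script do no effective work.
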(event Custom|CustomEvent_0
  (params (InNewParam :type Boolean) (InNewParam2 :type Byte) (InNewParam3 :type Float%20%28single-precision%29) (InNewParam4 :type Name))
  ;[0.1991 0.1606 0.8333] Event
  (Development|PrintString (Utilities|String|ToString(Boolean) InNewParam) true true (Math|Color|SelectColor "(R=0.133852,G=0.583333,B=0.000000,A=1.000000)" "(R=0.567708,G=0.000000,B=0.014453,A=1.000000)" InNewParam) 5.0))

(event Custom|CustomEvent_1)

(event EventBeginPlay
  ;[0.2705 0.9801 1] Logic
  (CallFunction|CustomEvent0 false 0 0.0 "None")
  (CallFunction|CustomEvent0 true 0 0.0 "None"))

(event Collision|EventActorBeginOverlap
  (params (OtherActor :type Actor%20Object%20Reference)))

(event EventTick
  (params (DeltaSeconds :type Float%20%28single-precision%29)))

(fn ConstructionScript)

(fn NewFunction0
  (params (InName :type Name) (InArray :type Array%20of%20Booleans) (InInt :type Integer))
  (bind _output (Utilities|Array|Get(acopy) InArray))
  (Utilities|FlowControl|Sequence
    (:then_1)
    (:then_4
      (if _output
        (CallFunction|CustomEvent0 _output 0 (Math|Conversions|ToFloat(Integer) InInt) InName)
        (CallFunction|CustomEvent1)
        (Test|NewFunction0 "None" (Utilities|Array|MakeArray false))))))

(fn NewFunction1)